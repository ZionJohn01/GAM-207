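; Player projectile actor that damages AI characters on contact and expires on its own after a few seconds.
; An overlap with an AI character passes through a DoOnce so only the first hit applies damage, credited to the projectile's owner.
; The hit spawns an impact particle system at the target with randomized yaw, then destroys the projectile after a short delay.
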(event OnComponentBeginOverlap(ProjectileOverlap)
  (params (OverlappedComponent :type Primitive%20Component%20Object%20Reference) (OtherActor :type Actor%20Object%20Reference) (OtherComp :type Primitive%20Component%20Object%20Reference) (OtherBodyIndex :type Integer) (bFromSweep :type Boolean) (SweepResult :type Hit%20Result%20Structure%20%28by%20ref%29))
  (bind _asaicharacter_bp (Utilities|Casting|CastToAICharacter_BP OtherActor))
  (Utilities|FlowControl|DoOnce false
    (:Completed
      (Game|Damage|ApplyDamage _asaicharacter_bp 25.0 0 (Components|GetOwner))
      (Niagara|SpawnSystematLocation "/Game/Player/Projectile/ProjectileHit.ProjectileHit" (Transformation|GetActorLocation _asaicharacter_bp) (Math|Rotator|MakeRotator (.Roll (Math|Rotator|BreakRotator (Transformation|GetActorRotation _asaicharacter_bp))) (.Pitch (Math|Rotator|BreakRotator (Transformation|GetActorRotation _asaicharacter_bp))) (+ (.Yaw (Math|Rotator|BreakRotator (Transformation|GetActorRotation _asaicharacter_bp))) (Math|Random|RandomFloatinRange 0.0 9e+01))))
      (Utilities|FlowControl|Delay 0.2)
      (Actor|DestroyActor))))

(event EventBeginPlay
  (Utilities|FlowControl|Delay 3.0)
  (Actor|DestroyActor))

(fn ConstructionScript)