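; AI projectile actor that damages AI characters and the player on overlap, and destroys itself three seconds after spawning if still alive.
; AI characters are hit only through their capsule, spawning a hit effect with randomized yaw before a short delayed destroy.
; Player overlaps apply the same damage, credited to the owner, and destroy it immediately without an effect.
; Each branch has its own DoOnce gate against repeated damage.
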(event OnComponentBeginOverlap(ProjectileOverlap)
  (params (OverlappedComponent :type Primitive%20Component%20Object%20Reference) (OtherActor :type Actor%20Object%20Reference) (OtherComp :type Primitive%20Component%20Object%20Reference) (OtherBodyIndex :type Integer) (bFromSweep :type Boolean) (SweepResult :type Hit%20Result%20Structure%20%28by%20ref%29))
  (bind _returnvalue (Components|GetOwner))
  (bind _asaicharacter_bp (Utilities|Casting|CastToAICharacter_BP OtherActor)
    (:then
      (if (== OtherComp (Variables|/Script/Engine.Character|GetCapsuleComponent _asaicharacter_bp))
        (Utilities|FlowControl|DoOnce false
          (:Completed
            (Game|Damage|ApplyDamage _asaicharacter_bp 1e+01 0 _returnvalue)
            (Niagara|SpawnSystematLocation "/Game/Player/Projectile/ProjectileHit.ProjectileHit" (Transformation|GetActorLocation _asaicharacter_bp) (Math|Rotator|MakeRotator (.Roll (Math|Rotator|BreakRotator (Transformation|GetActorRotation _asaicharacter_bp))) (.Pitch (Math|Rotator|BreakRotator (Transformation|GetActorRotation _asaicharacter_bp))) (+ (.Yaw (Math|Rotator|BreakRotator (Transformation|GetActorRotation _asaicharacter_bp))) (Math|Random|RandomFloatinRange 0.0 9e+01))))
            (Utilities|FlowControl|Delay 0.2)
            (Actor|DestroyActor :!label _label)))))
    (:CastFailed
      (bind _asplayer_character_bp (Utilities|Casting|CastToPlayerCharacter_BP OtherActor))
      (Utilities|FlowControl|DoOnce false
        (:Completed
          (Game|Damage|ApplyDamage _asplayer_character_bp 1e+01 0 _returnvalue)
          (goto _label))))))

(event EventBeginPlay
  (Utilities|FlowControl|Delay 3.0)
  (Actor|DestroyActor))

(fn ConstructionScript)